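; GA_Sprint is a Gameplay Ability that makes the owning character sprint at a higher walk speed.
; On activation it applies the GE_SprintDrain effect, stores its handle, and raises the CharacterMovement MaxWalkSpeed.
; A WaitGameplayEvent on Ability.StopSprint removes the drain, sets walk speed back to a hardcoded value and ends the ability.
; OnEndAbility is empty, so cleanup happens only on that event path.
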(event `self.K2_ActivateAbility`
  (bind _returnvalue (`self.BP_ApplyGameplayEffectToOwner` "/Game/Genesis/GAS/Effects/GE_SprintDrain.GE_SprintDrain_C"))
  (set `self.DrainEffectHandle` _returnvalue)
  (bind _ascharacter (cast `Character` (`self.GetAvatarActorFromActorInfo`)))
  (bind _charactermovement (`Character.CharacterMovement` _ascharacter))
  (set `CharacterMovementComponent.MaxWalkSpeed` 800.0 _charactermovement)
  (`AbilityTask_WaitGameplayEvent.WaitGameplayEvent` (struct :`TagName` "Ability.StopSprint") null
    (:`EventReceived`
      (`self.BP_RemoveGameplayEffectFromOwnerWithHandle` (`self.DrainEffectHandle`))
      (set `CharacterMovementComponent.MaxWalkSpeed` 500.0 _charactermovement)
      (`self.K2_EndAbility`))))